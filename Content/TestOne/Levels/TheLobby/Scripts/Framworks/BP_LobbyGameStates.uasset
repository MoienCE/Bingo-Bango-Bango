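; Lobby state Blueprint that tracks a state per ID and broadcasts whether the first two match.
; On BeginPlay it caches the default HUD and binds to the first Spawner's spawn event, which fills the States array with 3 as an unset sentinel.
; Update writes a state by ID and, once no sentinel remains, fires OnEqualityChanged with the comparison of the first two entries.
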(event `self.ReceiveBeginPlay`
  (bind _ashud_default (cast `/Game/TestOne/Levels/TheLobby/Scripts/Framworks/HUD_Default` (`PlayerController.GetHUD` (`GameplayStatics.GetPlayerController` 0))))
  (set `self.HUD_Reference` _ashud_default)
  (bind _outactors (`GameplayStatics.GetAllActorsOfClass` "/Game/TestOne/Levels/TheLobby/Scripts/Framworks/Spawner.Spawner_C"))
  (add `/Game/TestOne/Levels/TheLobby/Scripts/Framworks/Spawner.on_spawned` (`|GetArrayItem` _outactors) (delegate `on_spawned_Event`)))

(event `on_spawned_Event`
  (params (count :type Integer))
  (set `self.States` (`|MakeArray`))
  (for _ (range 1 (+ count 1))
    (`KismetArrayLibrary.Array_Add` (`self.States`) 3)))

(fn `Update`
  (params (ID :type Integer) (NewState :type Integer))
  (bind _states (`self.States`))
  (`KismetArrayLibrary.Array_Set` _states ID NewState)
  (for _array_element (`self.States`)
    (if (== _array_element 3)
      (set `self.all_changed` false)
      (break)))
  (if (`self.all_changed`)
    (`KismetSystemLibrary.PrintString` "equaliti changed")
    (if (== (`|GetArrayItem` _states) (`|GetArrayItem` _states 1))
      (set `self.isEq` true)
      (else
        (set `self.isEq` false)))
    (`self.on equality changed` (`self.isEq`))
    (else
      (set `self.all_changed` true))))

(fn `UserConstructionScript`)