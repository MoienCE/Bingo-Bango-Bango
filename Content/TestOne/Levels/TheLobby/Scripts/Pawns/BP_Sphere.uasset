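; BP_Sphere is a clickable sphere in TheLobby level that changes to a random material and reports its state to the game state.
; Hovering switches the mouse cursor to a hand and back to default on exit.
; A click picks a random index for one of three materials, applies it to Body, then passes the sphere's ID and new State to BP_LobbyGameStates.
; The construction script starts State outside that random range.
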(event `self.ReceiveActorEndCursorOver`
  ;[0.1 0.2 0.2] Change Mouse Cursor on overlap
  (set `PlayerController.CurrentMouseCursor` "Default" (`GameplayStatics.GetPlayerController` 0)))

(event `self.ReceiveActorBeginCursorOver`
  ;[0.1 0.2 0.2] Change Mouse Cursor on overlap
  (set `PlayerController.CurrentMouseCursor` "Hand" (`GameplayStatics.GetPlayerController` 0)))

(event `self.ReceiveActorOnClicked`
  (params (ButtonPressed :type "Key Structure"))
  ;[0.05 0.1 0.2] changing material
  (`self.Chose_Random_material`)
  ;[0.2 0.1 0.5] update game state
  (bind _asbp_lobby_game_states (cast `/Game/TestOne/Levels/TheLobby/Scripts/BP_LobbyGameStates` (`GameplayStatics.GetGameState`)))
  (`/Game/TestOne/Levels/TheLobby/Scripts/BP_LobbyGameStates.update` _asbp_lobby_game_states (`self.ID`) (`self.state`)))

(fn `Chose_Random_material`
  (bind _output_get (set `self.state` (`KismetMathLibrary.RandomIntegerInRange` 0 2)))
  (`PrimitiveComponent.SetMaterial` (`self.body`) 0 (`|GetArrayItem` (`self.materials`) _output_get)))

(fn `UserConstructionScript`
  (set `self.state` 4))