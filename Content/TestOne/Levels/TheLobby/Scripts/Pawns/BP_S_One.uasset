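; BP_S_One is a clickable lobby Blueprint that changes its Body material at random when clicked.
; Cursor overlap events switch the first player controller's mouse cursor to a hand on hover and back to default on exit.
; A click calls ChoseRandomMaterial, which picks one of the first three entries in the Materials array and applies it to Body's first material slot.
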(event `self.ReceiveBeginPlay`)

(event `self.ReceiveActorEndCursorOver`
  ;[0.1 0.2 0.2] Change Mouse Cursor on overlap
  (set `PlayerController.CurrentMouseCursor` "Default" (`GameplayStatics.GetPlayerController` 0)))

(event `self.ReceiveActorBeginCursorOver`
  ;[0.1 0.2 0.2] Change Mouse Cursor on overlap
  (set `PlayerController.CurrentMouseCursor` "Hand" (`GameplayStatics.GetPlayerController` 0)))

(event `self.ReceiveActorOnClicked`
  (params (ButtonPressed :type "Key Structure"))
  (`self.Chose_Random_material`))

(fn `Chose_Random_material`
  (`PrimitiveComponent.SetMaterial` (`self.body`) 0 (`|GetArrayItem` (`self.materials`) (`KismetMathLibrary.RandomIntegerInRange` 0 2))))

(fn `UserConstructionScript`)